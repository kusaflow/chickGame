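; Poo power-up pickup block that boosts the chick character's double jump power.
; When the chick overlaps the static mesh, it raises that power by a fixed amount and sets the PooMterAnim flag on kusaGameInstance.
; It then spawns an emitter and plays a sound at the Box component's location, and destroys itself.
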(event `self.StaticMesh.OnComponentBeginOverlap`
  (params (OverlappedComponent :type "PrimitiveComponent Object Reference") (OtherActor :type "Actor Object Reference") (OtherComp :type "PrimitiveComponent Object Reference") (OtherBodyIndex :type Integer) (bFromSweep :type Boolean) (SweepResult :type "HitResult Structure (by ref)"))
  (bind _returnvalue (`SceneComponent.K2_GetComponentLocation` (`self.Box`)))
  (bind _aschick (cast `chick` OtherActor))
  (bind _askusa_game_instance (cast `kusaGameInstance` (`GameplayStatics.GetGameInstance`)))
  (set `kusaGameInstance.pooMterAnim` true _askusa_game_instance)
  (set `chick.doubleJumpPower` (+ (`chick.doubleJumpPower` _aschick) 50.0) _aschick)
  (`GameplayStatics.SpawnEmitterAtLocation` "/Game/utils/danger.danger" _returnvalue)
  (`GameplayStatics.PlaySoundAtLocation` "/Game/sound/poo.poo" _returnvalue (struct) 1.0 1.0 0.0 null null null)
  (`self.K2_DestroyActor`))

(fn `UserConstructionScript`)